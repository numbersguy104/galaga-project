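; BP_Bullet is a projectile that travels straight up the world Z axis and destroys enemies it touches.
; Tick moves it by a fixed speed scaled by delta time, without sweeping, and destroys it once it passes a height limit.
; On actor overlap, an exact class match against BP_Enemy destroys both the enemy and the bullet.
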(event EventBeginPlay)

(event Collision|EventActorBeginOverlap
  (params (OtherActor :type Actor%20Object%20Reference))
  ;[0.15 0.15 0.15 0.5] Destroy enemies the bullet touches
  (if (== (Utilities|GetClass OtherActor) "/Game/Blueprints/BP_Enemy.BP_Enemy_C")
    (Actor|DestroyActor OtherActor)
    (Actor|DestroyActor)))

(event EventTick
  (params (DeltaSeconds :type Float%20%28single-precision%29))
  (bind _returnvalue (Transformation|GetActorLocation))
  (bind (_x _y _z) (Math|Vector|BreakVector _returnvalue))
  (Transformation|SetActorLocation (Math|Vector|MakeVector _x _y (+ _z (* 1e+03 DeltaSeconds))) false false)
  (if (> _z 2e+03)
    (Actor|DestroyActor)))

(fn ConstructionScript)