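; BP_NewPlayer is a player-controlled Blueprint that slides along the world X axis and spawns an actor on Space Bar.
; Tick offsets the X location by the MoveRight axis value, Speed and delta time, setting it directly without sweep collision.
; Space Bar spawns the actor at the player's current transform; the file does not show which class is spawned.
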(event EventBeginPlay)

(event Collision|EventActorBeginOverlap
  (params (OtherActor :type Actor%20Object%20Reference)))

(event EventTick
  (params (DeltaSeconds :type Float%20%28single-precision%29))
  (bind _returnvalue (Transformation|GetActorLocation))
  (bind (_x _y _z) (Math|Vector|BreakVector _returnvalue))
  (Transformation|SetActorLocation (Math|Vector|MakeVector (+ _x (* (stale Input|AxisEvents|InputAxisMoveRight AxisValue) DeltaSeconds (Variables|Default|GetSpeed))) _y _z) false false))

(event Input|AxisEvents|InputAxisMoveRight
  (params (AxisValue :type Float%20%28single-precision%29)))

(event Input|KeyboardEvents|SpaceBar
  (params (Key :type Key%20Structure :default "None"))
  (:Pressed
    (Game|SpawnActorfromClass "/Game/Blueprints/BP_Bullet.BP_Bullet_C" (Transformation|GetActorTransform) "Undefined" "MultiplyWithRoot" 0 0)))

(fn ConstructionScript)